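; BP_MeshActor is a mesh prop that swaps its static mesh for a procedural mesh copy at runtime.
; The construction script picks the mesh from an override or a Shape choice such as stone, barrel or shield.
; BeginPlay copies it into the procedural mesh with collision and destroys the static mesh component.
; Randomly spawned instances get random rotation and scale, are launched by an impulse, and lose their mesh after ten seconds.
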(event `self.ReceiveBeginPlay`
  ;[0.36 0 0] Begin Play
  (`StaticMeshComponent.SetStaticMesh` (`self.StaticMesh`) (`self.Get Static Mesh By Shape Type`))
  (`SceneComponent.K2_SetRelativeTransform` (`self.ProceduralMesh`) (`SceneComponent.GetRelativeTransform` (`self.StaticMesh`)) false false)
  (`KismetProceduralMeshLibrary.CopyProceduralMeshFromStaticMeshComponent` (`self.StaticMesh`) 0 (`self.ProceduralMesh`) true)
  (`ActorComponent.K2_DestroyComponent` (`self.StaticMesh`))
  (if (`self.Is Randomly Spawned ?`)
    (`SceneComponent.K2_SetRelativeTransform` (`self.ProceduralMesh`) (`KismetMathLibrary.MakeTransform` (`SceneComponent.RelativeLocation` (`self.ProceduralMesh`)) (`KismetMathLibrary.RandomRotator` true) (`KismetMathLibrary.Conv_DoubleToVector` (`KismetMathLibrary.RandomFloatInRange` 0.5 1.2))) false false)
    (`PrimitiveComponent.AddImpulse` (`self.ProceduralMesh`) (`KismetMathLibrary.MakeVector` -400.0 (`KismetMathLibrary.RandomFloatInRange` -100.0 100.0) 1000.0) "None" true)
    (`KismetSystemLibrary.Delay` 10.0)
    (`ActorComponent.K2_DestroyComponent` (`self.ProceduralMesh`))))

(fn `Get Static Mesh By Shape Type`
  (returns (ReturnValue :type "StaticMesh Object Reference"))
  (return (select `bool` (`KismetSystemLibrary.IsValid` (`self.Static Mesh Override`)) :`false` (select `byte` (`self.Shape`) :`0` "/Game/MedievalLevel/Assets/Stones/stone.Stone" :`1` "/Game/MedievalLevel/Assets/Barrel/barrel.Barrel" :`2` "/Game/MedievalLevel/Weapons/RoundShield/RoundShield.RoundShield" :`3` "/Game/MedievalLevel/Assets/Vase/DR20_Sealed.DR20_Sealed" :!type "StaticMesh Object Reference") :`true` (`self.Static Mesh Override`))))

(fn `UserConstructionScript`
  (`StaticMeshComponent.SetStaticMesh` (`self.StaticMesh`) (`self.Get Static Mesh By Shape Type`)))