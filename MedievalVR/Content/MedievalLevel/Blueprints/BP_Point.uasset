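; BP_Point is a score counter actor that shows an integer on a text render component.
; The UpValue event increments the counter and refreshes the displayed text.
; When a Blade actor ends its overlap with the TriggerBox_Slot level actor or component, the counter returns to zero and the text updates.
; The Reset event has no logic.
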(event `UpValue`
  (bind _output_get (set `self.Counter` (+ (`self.Counter`) 1)))
  (`TextRenderComponent.K2_SetText` (`self.TextRender`) (`KismetTextLibrary.Conv_IntToText` _output_get)))

(event `Reset`)

(event `self.TriggerBox_Slot.OnActorEndOverlap`
  (params (OverlappedActor :type "Actor Object Reference") (OtherActor :type "Actor Object Reference"))
  (cast `/Game/MedievalLevel/Blueprints/Blade` OtherActor)
  (bind _output_get (set `self.Counter` 0))
  (`TextRenderComponent.K2_SetText` (`self.TextRender`) (`KismetTextLibrary.Conv_IntToText` _output_get)))

(fn `UserConstructionScript`)